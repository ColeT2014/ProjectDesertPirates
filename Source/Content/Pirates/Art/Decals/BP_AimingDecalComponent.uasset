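; Decal component that sets up port and starboard aiming decals for a pirate ship.
; Initialize takes a Ship and spawns two large M_Decal decals attached to its root, offset along the negative and positive actor right vector and rotated to mirror each other.
; Both are stored as PortDecal and StarboardDecal and start hidden; this graph contains no logic to show them or update them per frame.
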(event EventBeginPlay)

(event EventTick
  (params (DeltaSeconds :type Float%20%28single-precision%29)))

(fn Initialize
  (params (Ship :type BP%20Ship%20Object%20Reference))
  (bind _returnvalue (Class|GameplayStatics|SpawnDecalAttached "/Game/Pirates/Art/Decals/M_Decal.M_Decal" "5120.000000,5120.000000,5120.000000" (Variables|/Script/Engine.Actor|GetRootComponent Ship) "None" (* (Math|Vector|NegateVector (Transformation|GetActorRightVector Ship)) 5e+03) "-90.000000,0.000000,0.000000" "KeepRelativeOffset" 0.0))
  (bind _output_get (Variables|Default|SetPortDecal _returnvalue))
  (Rendering|SetVisibility _output_get false false)
  (bind _returnvalue_2 (Class|GameplayStatics|SpawnDecalAttached "/Game/Pirates/Art/Decals/M_Decal.M_Decal" "5120.000000,5120.000000,5120.000000" (Variables|/Script/Engine.Actor|GetRootComponent Ship) "None" (* (Transformation|GetActorRightVector Ship) 5e+03) "-90.000000,180.000000,0.000000" "KeepRelativeOffset" 0.0))
  (bind _output_get_2 (Variables|Default|SetStarboardDecal _returnvalue_2))
  (Rendering|SetVisibility _output_get_2 false false))