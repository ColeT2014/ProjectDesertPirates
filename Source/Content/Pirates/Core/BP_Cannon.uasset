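; BP_Cannon is a ship or emplacement cannon actor that fires a projectile after a short randomized delay.
; SetTimer stores the velocity and instigator, then schedules Fire by name, using the absolute value of a roughly normal random delay.
; CLTNormalDistribution approximates that bell curve by summing three uniform random floats.
; Fire spawns a BP_Projectile_Parent at the cannon's transform with the stored values and plays the cannon sound.
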(event EventBeginPlay)

(event Collision|EventActorBeginOverlap
  (params (OtherActor :type Actor%20Object%20Reference)))

(event EventTick
  (params (DeltaSeconds :type Float%20%28single-precision%29)))

(fn ConstructionScript)

(fn SetTimer
  (params (Velocity :type Vector) (InstigatorRef :type Pawn%20Object%20Reference))
  (Variables|Default|SetVelocity Velocity)
  (Variables|Default|SetInstigatorRef InstigatorRef)
  (bind _returnvalue (Utilities|Time|SetTimerbyFunctionName 0 "Fire" (Math|Float|Absolute(Float) (CallFunction|CLTNormalDistribution 0.5 1.0))))
  (Variables|Default|SetFireTimer _returnvalue))

(fn Fire
  (Game|SpawnActorfromClass "/Game/Pirates/Core/BP_Projectile_Parent.BP_Projectile_Parent_C" (Transformation|GetActorTransform) "AlwaysSpawn" "OverrideRootScale" 0 (Variables|Default|GetVelocity) (Variables|Default|GetInstigatorRef))
  (Audio|PlaySoundatLocation (Variables|Default|GetCannonSound) (Transformation|GetWorldLocation (Variables|Default|GetDefaultSceneRoot)) "0, 0, 0" 1.0 1.0 0.0 0 0 0 0))

(fn CLTNormalDistribution
  (params (Mean :type Float%20%28double-precision%29) (StandardDeviation :type Float%20%28double-precision%29))
  (LocalVariables|SetS (+ (Math|Random|RandomFloatinRange 0.0 1.0) (Math|Random|RandomFloatinRange 0.0 1.0) (Math|Random|RandomFloatinRange 0.0 1.0)))
  (bind _output_get (LocalVariables|SetN (+ Mean (* StandardDeviation (- (LocalVariables|GetS) 1.5)))))
  (return _output_get))