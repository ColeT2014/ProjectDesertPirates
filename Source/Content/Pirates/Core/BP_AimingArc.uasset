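; BP_AimingArc is an actor that draws an aiming arc as a chain of spline meshes along its Spline component.
; UpdateSpline destroys the previous meshes, then adds one manually attached spline mesh per segment using world-space points and tangents.
; Each segment's start and end scale shrinks linearly with point index, so the arc tapers toward its far end.
; The spline points are not set in this graph.
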(event EventBeginPlay)

(fn ConstructionScript)

(fn UpdateSpline
  (bind _spline (Variables|Default|GetSpline))
  (bind _spline_2 (Variables|Default|GetSpline))
  (bind _spline_3 (Variables|Default|GetSpline))
  (bind _splinemeshes (Variables|Default|GetSplineMeshes))
  (bind _returnvalue (Spline|GetNumberOfSplinePoints _spline_3))
  (bind _returnvalue_2 (Spline|GetNumberOfSplinePoints _spline_2))
  (bind _returnvalue_3 (Math|Conversions|ToFloat(Integer) _returnvalue))
  (Components|DestroyComponent _splinemeshes)
  (Utilities|Array|Clear _splinemeshes)
  (for _index (range 0 (- (Spline|GetNumberOfSplinePoints (Variables|Default|GetSpline)) 2))
    (LocalVariables|Seti _index)
    (bind _returnvalue_4 (AddComponent|AddSplineMeshComponent true))
    (bind _output_get (LocalVariables|SetCurrentSplineMesh _returnvalue_4))
    (Utilities|Array|Add (Variables|Default|GetSplineMeshes) _output_get)
    (SplineMesh|SetStartandEnd (LocalVariables|GetCurrentSplineMesh) (.Location (Spline|GetLocationandTangentatSplinePoint _spline (LocalVariables|Geti) "World")) (.Tangent (Spline|GetLocationandTangentatSplinePoint _spline (LocalVariables|Geti) "World")) (.Location (Spline|GetLocationandTangentatSplinePoint _spline (+ (LocalVariables|Geti) 1) "World")) (.Tangent (Spline|GetLocationandTangentatSplinePoint _spline (+ (LocalVariables|Geti) 1) "World")) true :!class /Script/Engine.SplineMeshComponent)
    (SplineMesh|SetStartScale (LocalVariables|GetCurrentSplineMesh) (Math|Vector2D|MakeVector2D (/ (Math|Conversions|ToFloat(Integer) (- _returnvalue_2 (LocalVariables|Geti))) _returnvalue_3) (/ (Math|Conversions|ToFloat(Integer) (- _returnvalue_2 (LocalVariables|Geti))) _returnvalue_3)) true :!class /Script/Engine.SplineMeshComponent)
    (SplineMesh|SetEndScale (LocalVariables|GetCurrentSplineMesh) (Math|Vector2D|MakeVector2D (/ (Math|Conversions|ToFloat(Integer) (- _returnvalue_2 (+ (LocalVariables|Geti) 1))) _returnvalue_3) (/ (Math|Conversions|ToFloat(Integer) (- _returnvalue_2 (+ (LocalVariables|Geti) 1))) _returnvalue_3)) true :!class /Script/Engine.SplineMeshComponent)))