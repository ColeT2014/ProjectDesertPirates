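; BP_HealthComponent is a component that tracks separate hull and sail health for its owning actor in a pirate game.
; Both values start at their maximums on BeginPlay, and damage functions reduce them with a floor of zero.
; Zero hull destroys the owner, while the zero-sail branch is empty.
; Heal functions use Max rather than Min, so they raise health to at least the maximum instead of capping it.
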(event EventBeginPlay
  (Variables|Default|SetHull_Current (Variables|Default|GetHull_Max))
  (Variables|Default|SetSail_Current (Variables|Default|GetSail_Max)))

(event EventTick
  (params (DeltaSeconds :type Float%20%28single-precision%29)))

(fn TakeDamageHull
  (params (Damage :type Float%20%28double-precision%29))
  (bind _output_get (Variables|Default|SetHull_Current (Math|Float|Max(Float) (- (Variables|Default|GetHull_Current) Damage) 0.0)))
  (if (== _output_get 0.0)
    (Actor|DestroyActor (Components|GetOwner))))

(fn TakeDamageSail
  (params (Damage :type Float%20%28double-precision%29))
  (bind _output_get (Variables|Default|SetSail_Current (Math|Float|Max(Float) (- (Variables|Default|GetSail_Current) Damage) 0.0)))
  (if (== _output_get 0.0)
    _))

(fn HealDamageSail
  (params (Damage :type Float%20%28double-precision%29))
  (Variables|Default|SetSail_Current (Math|Float|Max(Float) (+ (Variables|Default|GetSail_Current) Damage) (Variables|Default|GetSail_Max))))

(fn HealDamageHull
  (params (Damage :type Float%20%28double-precision%29))
  (Variables|Default|SetHull_Current (Math|Float|Max(Float) (+ (Variables|Default|GetHull_Current) Damage) (Variables|Default|GetHull_Max))))