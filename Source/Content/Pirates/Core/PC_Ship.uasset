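; Player controller for a pirate ship that handles sail toggles, rudder steering, camera look and broadside firing.
; BeginPlay caches the ship and wind, spawns an aiming arc and adds health bar widgets.
; While aiming, the cursor's angle picks a hull quadrant, and the suggested toss velocity is clamped to that quadrant's firing limits and drawn as a predicted spline arc.
; Tick also drifts the camera toward the cursor and prints debug info.
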(event EventBeginPlay
  (CallFunction|Initialize))

(event EventTick
  (params (DeltaSeconds :type Float%20%28single-precision%29))
  (Variables|Default|SetTime DeltaSeconds)
  (CallFunction|PrintDebugInfo)
  (CallFunction|UpdateCameraOffset)
  (if (Variables|Default|GetbAiming)
    (CallFunction|TraceCursorLocation)
    (CallFunction|FindAimQuadrant)
    (bind _tossvelocity (Class|GameplayStatics|BlueprintSuggestProjectileVelocity (Transformation|GetActorLocation (Variables|Default|GetPlayerPawn)) (Variables|Default|GetCursorLocation) 1e+04 0.0 "DoNotTrace" 5e+01 false false))
    (Variables|Default|SetAimDirection (Math|Transform|InverseTransformDirection (Transformation|GetWorldTransform (Variables|/Game/Pirates/Core/BP_Ship.BP_Ship_C|GetHull (Variables|Default|GetPlayerPawn))) (Math|Vector|Normalize _tossvelocity)))
    (Variables|Default|SetReferenceVector (Utilities|Select :Index (Variables|Default|GetAimQuadrant) :NewEnumerator0 "0, 0, 0" :NewEnumerator1 "1.000000,0.000000,0.000000" :NewEnumerator2 "0.000000,1.000000,0.000000" :NewEnumerator3 "-1.000000,0.000000,0.000000" :NewEnumerator4 "0.000000,-1.000000,0.000000"))
    (Variables|Default|SetHorizontalAngle (Class|KismetMathLibrary|DegAtan2 (.z (Math|Vector|CrossProduct (Variables|Default|GetReferenceVector) (Variables|Default|GetAimDirection))) (Math|Vector|DotProduct (Variables|Default|GetReferenceVector) (Variables|Default|GetAimDirection))))
    (Variables|Default|SetVerticalAngle (Class|KismetMathLibrary|DegAtan2 (Utilities|Select :Index (Variables|Default|GetAimQuadrant) :NewEnumerator0 0.0 :NewEnumerator1 (* (.y (Math|Vector|CrossProduct (Variables|Default|GetReferenceVector) (Variables|Default|GetAimDirection))) -1.0) :NewEnumerator2 (.x (Math|Vector|CrossProduct (Variables|Default|GetReferenceVector) (Variables|Default|GetAimDirection))) :NewEnumerator3 (.y (Math|Vector|CrossProduct (Variables|Default|GetReferenceVector) (Variables|Default|GetAimDirection))) :NewEnumerator4 (* (.x (Math|Vector|CrossProduct (Variables|Default|GetReferenceVector) (Variables|Default|GetAimDirection))) -1.0)) (Math|Vector|DotProduct (Variables|Default|GetReferenceVector) (Variables|Default|GetAimDirection))))
    (Development|PrintString (Utilities|String|Append "HorizontalAngle: " (Utilities|String|ToString(Float) (Variables|Default|GetHorizontalAngle))) true true "(R=0.000000,G=0.660000,B=1.000000,A=1.000000)" 0.0)
    (Development|PrintString (Utilities|String|Append "VerticalAngle:" (Utilities|String|ToString(Float) (Variables|Default|GetVerticalAngle))) true true "(R=0.000000,G=0.660000,B=1.000000,A=1.000000)" 0.0)
    (Variables|Default|SetVerticalAngle (Math|Float|ClampAngle (Variables|Default|GetVerticalAngle) 0.0 2e+01))
    (Variables|Default|SetHorizontalAngle (Math|Float|ClampAngle (Variables|Default|GetHorizontalAngle) -1e+01 1e+01))
    (Variables|Default|SetAimDirection (* (Math|Vector|RotateVectorAroundAxis (Math|Vector|RotateVectorAroundAxis (Variables|Default|GetReferenceVector) (Variables|Default|GetVerticalAngle) (Utilities|Select :Index (Variables|Default|GetAimQuadrant) :NewEnumerator0 "0, 0, 0" :NewEnumerator1 "0.000000,-1.000000,0.000000" :NewEnumerator2 "1.000000,0.000000,0.000000" :NewEnumerator3 "0.000000,1.000000,0.000000" :NewEnumerator4 "-1.000000,0.000000,0.000000")) (Variables|Default|GetHorizontalAngle) "0.000000,0.000000,1.000000") 1e+04))
    (bind _outpathpositions (Class|GameplayStatics|BlueprintPredictProjectilePathbyObjectType (Transformation|GetActorLocation (Variables|Default|GetPlayerPawn)) (Math|Transform|TransformDirection (Transformation|GetWorldTransform (Variables|/Game/Pirates/Core/BP_Ship.BP_Ship_C|GetHull (Variables|Default|GetPlayerPawn))) (Variables|Default|GetAimDirection)) true 5e+01 (Utilities|Array|MakeArray "ObjectTypeQuery1") false (Utilities|Array|MakeArray (Variables|Default|GetPlayerPawn)) "None" 0.0 5.0 3.0))
    (Spline|SetSplinePoints (Variables|/Game/Pirates/Core/BP_AimingArc.BP_AimingArc_C|GetSpline (Variables|Default|GetAimingArc)) _outpathpositions "World" true)
    (Default|UpdateSpline (Variables|Default|GetAimingArc))
    (else
      (Spline|ClearSplinePoints (Variables|/Game/Pirates/Core/BP_AimingArc.BP_AimingArc_C|GetSpline (Variables|Default|GetAimingArc)) true)
      (Default|UpdateSpline (Variables|Default|GetAimingArc)))))

(event Input|ActionEvents|InputActionForesails
  (params (Key :type Key%20Structure :default "None"))
  (bind _playerpawn (Variables|Default|GetPlayerPawn))
  (:Pressed
    (switch Utilities|FlowControl|Switch|SwitchonE_SailsState (Variables|/Game/Pirates/Core/BP_Ship.BP_Ship_C|GetSailState (Variables|Default|GetPlayerPawn))
      (:NewEnumerator0
        (Default|SetSailState _playerpawn "NewEnumerator2"))
      (:NewEnumerator1
        (Default|SetSailState _playerpawn "NewEnumerator3"))
      (:NewEnumerator2
        (Default|SetSailState _playerpawn "NewEnumerator0"))
      (:NewEnumerator3
        (Default|SetSailState _playerpawn "NewEnumerator1")))))

(event Input|ActionEvents|InputActionAftsails
  (params (Key :type Key%20Structure :default "None"))
  (bind _playerpawn (Variables|Default|GetPlayerPawn))
  (:Pressed
    (switch Utilities|FlowControl|Switch|SwitchonE_SailsState (Variables|/Game/Pirates/Core/BP_Ship.BP_Ship_C|GetSailState (Variables|Default|GetPlayerPawn))
      (:NewEnumerator0
        (Default|SetSailState _playerpawn "NewEnumerator1"))
      (:NewEnumerator1
        (Default|SetSailState _playerpawn "NewEnumerator0"))
      (:NewEnumerator2
        (Default|SetSailState _playerpawn "NewEnumerator3"))
      (:NewEnumerator3
        (Default|SetSailState _playerpawn "NewEnumerator2")))))

(event Input|AxisEvents|InputAxisTurnRate
  (params (AxisValue :type Float%20%28single-precision%29))
  ;[0.1302 0.1302 0.1302] Gamepad/WASD input
  (Pawn|Input|AddControllerYawInput (Variables|Default|GetPlayerPawn) (* AxisValue (Variables|Default|GetBaseTurnRate) (Utilities|Time|GetWorldDeltaSeconds))))

(event Input|AxisEvents|InputAxisLookUpRate
  (params (AxisValue :type Float%20%28single-precision%29))
  ;[0.1302 0.1302 0.1302] Gamepad/WASD input
  (Pawn|Input|AddControllerPitchInput (Variables|Default|GetPlayerPawn) (* AxisValue (Variables|Default|GetBaseLookUpRate) (Utilities|Time|GetWorldDeltaSeconds))))

(event Input|AxisEvents|InputAxisMoveRight
  (params (AxisValue :type Float%20%28single-precision%29))
  (Variables|/Game/Pirates/Core/BP_Ship.BP_Ship_C|SetRudder (Variables|Default|GetPlayerPawn) (Math|Float|Clamp(Float) (+ (* AxisValue (Variables|/Game/Pirates/Core/BP_Ship.BP_Ship_C|GetRudderDelta (Variables|Default|GetPlayerPawn)) (Variables|Default|GetTime)) (Variables|/Game/Pirates/Core/BP_Ship.BP_Ship_C|GetRudder (Variables|Default|GetPlayerPawn))) -1.0)))

(event Input|KeyboardEvents|SpaceBar
  (params (Key :type Key%20Structure :default "None"))
  (:Pressed
    (Default|FireBroadSide (Variables|Default|GetPlayerPawn) (Variables|Default|GetAimQuadrant) (Variables|Default|GetAimDirection))))

(event Input|KeyboardEvents|Z
  (params (Key :type Key%20Structure :default "None"))
  (:Pressed
    (if (Variables|Default|GetbAiming)
      (Variables|Default|SetbAiming false)
      (else
        (Variables|Default|SetbAiming true)))))

(fn ConstructionScript)

(fn Initialize
  (Utilities|FlowControl|Sequence
    (:then_0
      (bind _asbp_ship (Utilities|Casting|CastToBP_Ship (Game|Player|GetPlayerPawn 0)))
      (Variables|Default|SetPlayerPawn _asbp_ship))
    (:then_1
      (bind _outactors (Actor|GetAllActorsOfClass "/Game/Pirates/Core/BP_Wind.BP_Wind_C"))
      (Variables|Default|SetWind (Utilities|Array|Get(acopy) _outactors)))
    (:then_2
      (Development|SetHiddeninGame (Variables|/Game/Pirates/Core/BP_Ship.BP_Ship_C|GetWindDirection (Variables|Default|GetPlayerPawn)) false false))
    (:then_3
      (bind _returnvalue (Game|SpawnActorfromClass "/Game/Pirates/Core/BP_AimingArc.BP_AimingArc_C" (Transformation|GetActorTransform (Variables|Default|GetPlayerPawn)) "AlwaysSpawn" "MultiplyWithRoot" 0 (Variables|Default|GetPlayerPawn) 0))
      (Variables|Default|SetAimingArc _returnvalue))
    (:then_4
      (bind _returnvalue_2 (UserInterface|CreateWidget "/Game/Pirates/UserInterface/Player/WBP_Player_Health_Bar.WBP_Player_Health_Bar_C"))
      (UserInterface|Viewport|AddtoViewport _returnvalue_2 0)
      (bind _outactors_2 (Actor|GetAllActorsOfClass "/Game/Pirates/Core/BP_Ship.BP_Ship_C"))
      (for _array_element _outactors_2
        (if (not (Pawn|IsPlayerControlled _array_element))
          (Variables|Default|SetTarget _array_element)))
      (bind _returnvalue_3 (UserInterface|CreateWidget "/Game/Pirates/UserInterface/NPC/WBP_NPC_Health_Bar.WBP_NPC_Health_Bar_C"))
      (UserInterface|Viewport|AddtoViewport _returnvalue_3 0))))

(fn PrintDebugInfo
  (Development|PrintString (Utilities|String|ToString(Float) (Variables|/Game/Pirates/Core/BP_Ship.BP_Ship_C|GetWindEffectiveness (Variables|Default|GetPlayerPawn))) true true "(R=1.000000,G=0.094654,B=0.000000,A=1.000000)" 0.0)
  (Development|PrintString (Utilities|String|ToString(Float) (Variables|/Game/Pirates/Core/BP_Ship.BP_Ship_C|GetTrueWindAngle (Variables|Default|GetPlayerPawn))) true true "(R=0.000000,G=0.660000,B=1.000000,A=1.000000)" 0.0)
  (Development|PrintString (Utilities|String|Append "Rudder: " (Utilities|String|ToString(Float) (Variables|/Game/Pirates/Core/BP_Ship.BP_Ship_C|GetRudder (Variables|Default|GetPlayerPawn)))) true true "(R=0.000000,G=0.660000,B=1.000000,A=1.000000)" 0.0)
  (Development|PrintString (Utilities|String|EnumtoString (Variables|/Game/Pirates/Core/BP_Ship.BP_Ship_C|GetSailState (Variables|Default|GetPlayerPawn))) true true "(R=0.000000,G=0.660000,B=1.000000,A=1.000000)" 0.0))

(fn UpdateCameraOffset
  (bind (_locationx _locationy) (Game|Player|GetMousePosition))
  (bind _returnvalue (Viewport|GetViewportSize))
  (bind _returnvalue_2 (Pawn|GetControlRotation :!class /Script/Engine.Controller))
  (bind _playerpawn (Variables|Default|GetPlayerPawn))
  (bind _returnvalue_3 (Math|Vector|GetForwardVector _returnvalue_2))
  (bind _returnvalue_4 (Math|Vector|GetRightVector _returnvalue_2))
  (bind _returnvalue_5 (/ _locationy (.y _returnvalue)))
  (bind _returnvalue_6 (/ _locationx (.x _returnvalue)))
  (bind _cameraboom (Variables|/Game/Pirates/Core/BP_Ship.BP_Ship_C|GetCameraBoom _playerpawn))
  (bind _returnvalue_7 (- _returnvalue_5 0.5))
  (bind _returnvalue_8 (- _returnvalue_6 0.5))
  (bind _returnvalue_9 (* _returnvalue_4 _returnvalue_8))
  (bind _returnvalue_10 (* _returnvalue_3 _returnvalue_7 -1.0))
  (bind _returnvalue_11 (+ _returnvalue_10 _returnvalue_9))
  (bind _returnvalue_12 (* _returnvalue_11 7e+03))
  (bind (_x _y) (Math|Vector|BreakVector _returnvalue_12))
  (Variables|/Script/Engine.SpringArmComponent|SetTargetOffset _cameraboom (Math|Interpolation|VInterpTo (Variables|/Script/Engine.SpringArmComponent|GetTargetOffset _cameraboom) (Math|Vector|MakeVector _x _y 0.0) (Variables|Default|GetTime) 1.0)))

(fn TraceCursorLocation
  (bind _array (Utilities|Array|MakeArray "ObjectTypeQuery1"))
  (bind _playerpawn (Variables|Default|GetPlayerPawn))
  (bind (_hitresult _returnvalue) (Class|PlayerController|GetHitResultUnderCursorforObjects _array true))
  (bind _returnvalue_2 (Transformation|GetActorForwardVector _playerpawn))
  (if _returnvalue
    (Variables|Default|SetCursorLocation (.Location (Collision|BreakHitResult _hitresult)))
    (Variables|Default|SetCursorAngle (Class|KismetMathLibrary|DegAtan2 (.z (Math|Vector|CrossProduct _returnvalue_2 (Math|Vector|GetUnitDirection(Vector) (* (Transformation|GetActorLocation (Variables|Default|GetPlayerPawn)) "1.000000,1.000000,0") (* (Variables|Default|GetCursorLocation) "1.000000,1.000000,0")))) (Math|Vector|DotProduct _returnvalue_2 (Math|Vector|GetUnitDirection(Vector) (* (Transformation|GetActorLocation (Variables|Default|GetPlayerPawn)) "1.000000,1.000000,0") (* (Variables|Default|GetCursorLocation) "1.000000,1.000000,0")))))))

(fn FindAimQuadrant
  (if (Math|Float|InRange(Float) (Variables|Default|GetCursorAngle) -45.0 45.0)
    (Variables|Default|SetAimQuadrant "NewEnumerator1")
    (elif (> (Math|Float|Absolute(Float) (Variables|Default|GetCursorAngle)) 135.0)
      (Variables|Default|SetAimQuadrant "NewEnumerator3")
      (elif (Math|Float|InRange(Float) (Variables|Default|GetCursorAngle) -135.0 -45.0)
        (Variables|Default|SetAimQuadrant "NewEnumerator4")
        (elif (Math|Float|InRange(Float) (Variables|Default|GetCursorAngle) 45.0 135.0)
          (Variables|Default|SetAimQuadrant "NewEnumerator2")
          (else
            (Variables|Default|SetAimQuadrant "NewEnumerator0")))))))