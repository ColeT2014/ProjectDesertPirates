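; BP_Wind is a wind actor that maintains a gradually changing WindVector and Strength.
; The construction script seeds the direction from the actor's forward vector and sizes an arrow by Strength.
; Each Tick advances two Perlin noise inputs: one incrementally rotates the vector around the up axis, the other remaps to strength.
; A timer-based random direction function exists but is never called from the event graph.
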(event EventBeginPlay)

(event Collision|EventActorBeginOverlap
  (params (OtherActor :type Actor%20Object%20Reference)))

(event EventTick
  (params (DeltaSeconds :type Float%20%28single-precision%29))
  (Variables|Default|SetTime DeltaSeconds)
  (Variables|Default|SetPerlin (+ (* (Variables|Default|GetTime) (Variables|Default|GetPerlinSpeed)) (Variables|Default|GetPerlin)))
  (Variables|Default|SetPerlin2 (+ (* (Variables|Default|GetTime) (Variables|Default|GetPerlin2Speed)) (Variables|Default|GetPerlin2)))
  (Variables|Default|SetStrength (Math|Float|MapRangeClamped (Class|KismetMathLibrary|PerlinNoise1D (Variables|Default|GetPerlin2)) -1.0 1.0 7.0 3e+01))
  (Variables|Default|SetWindVector (Math|Vector|RotateVectorAroundAxis (Variables|Default|GetWindVector) (* (Class|KismetMathLibrary|PerlinNoise1D (Variables|Default|GetPerlin)) (Variables|Default|GetPerlinScale)) (Math|Vector|VectorUp))))

(fn ConstructionScript
  (Variables|Default|SetWindVector (Transformation|GetActorForwardVector))
  (Transformation|SetWorldScale3D (Variables|Default|GetArrow) (Math|Conversions|ToVector(Float) (/ (Variables|Default|GetStrength) 1e+01))))

(fn ChooseNewWindDirection
  (Variables|Default|SetWindVector (Math|Vector|RotateVectorAroundAxis (Variables|Default|GetWindVector) (Math|Random|RandomFloatinRange -3e+01 3e+01) (Math|Vector|VectorUp)))
  (Utilities|Time|SetTimerbyFunctionName 0 "ChooseNewWindDirection" (Math|Random|RandomFloatinRange 1e+01 3e+01)))