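; Base projectile Blueprint for the pirate game, launched along its local start velocity through a ProjectileMovement component.
; On overlap with a valid actor it destroys itself, first applying damage if that actor has a BP_HealthComponent.
; ApplyDamage routes non-zero hull and sail damage to separate functions on that component.
; A quadratic drag calculation is present but disconnected, and a debug print remains on hits.
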(event EventBeginPlay
  (Game|Components|ProjectileMovement|SetVelocityinLocalSpace (Variables|Default|GetProjectileMovement) (Variables|Default|GetStartVelocity)))

(event EventTick
  (params (DeltaSeconds :type Float%20%28single-precision%29)))

(event Collision|EventActorBeginOverlap
  (params (OtherActor :type Actor%20Object%20Reference))
  (bind _returnvalue (Actor|GetComponentbyClass OtherActor "/Game/Pirates/Core/BP_HealthComponent.BP_HealthComponent_C"))
  (Utilities|IsValid OtherActor
    (:Is%20Valid
      (Utilities|IsValid _returnvalue
        (:Is%20Valid
          (CallFunction|ApplyDamage _returnvalue)
          (Development|PrintString "Hello")
          (Actor|DestroyActor))
        (:Is%20Not%20Valid
          (Actor|DestroyActor))))))

(fn ConstructionScript)

(fn ApplyDamage
  (params (HealthComponent :type BP%20Health%20Component%20Object%20Reference))
  (Utilities|FlowControl|Sequence
    (:then_0
      (if (!= (Variables|Default|GetHullDamage) 0.0)
        (Default|TakeDamageHull HealthComponent (Variables|Default|GetHullDamage))))
    (:then_1
      (if (!= (Variables|Default|GetSailDamage) 0.0)
        (Default|TakeDamageSail HealthComponent (Variables|Default|GetSailDamage))))))